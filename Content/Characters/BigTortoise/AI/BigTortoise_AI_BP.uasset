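; AI controller for the BigTortoise boss that runs its behavior tree and feeds it blackboard state.
; Sight perception stores the player as target, and Tick flags when the player is too far away.
; A once-per-second countdown on a blackboard timer ends the fight at zero, destroying both arena bounds, updating the player's HUD, awarding score and marking the fight as ended.
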(event `self.ReceiveTick`
  (params (DeltaSeconds :type "Float (single-precision)"))
  (bind _returnvalue (`GameplayStatics.GetPlayerCharacter` 0))
  (`/Engine/EditorBlueprintResources/StandardMacros.IsValid` _returnvalue
    (:`Is Valid`
      (`BlackboardComponent.SetValueAsBool` (`self.Blackboard`) "bPlayerTooFarAway" (> (`KismetMathLibrary.Vector_Distance` (`self.K2_GetActorLocation` _returnvalue) (`self.K2_GetActorLocation` (`self.K2_GetPawn`))) 1600.0)))))

(event `StartFightCountdown`
  (bind _returnvalue (`BlackboardComponent.GetValueAsInt` (`AIBlueprintHelperLibrary.GetBlackboard` (`self.K2_GetPawn`)) "FightSecondsLeft"))
  (`KismetSystemLibrary.Delay` 1.0)
  (if (> _returnvalue 0) :!label _label
    (bind _result (`/Engine/EditorBlueprintResources/StandardMacros.DecrementInt` _returnvalue)
      (:`  `
        (`BlackboardComponent.SetValueAsInt` (`AIBlueprintHelperLibrary.GetBlackboard` (`self.K2_GetPawn`)) "FightSecondsLeft" _result)
        (`KismetSystemLibrary.Delay` 1.0)
        (goto _label)))
    (else
      (`self.EndBossFight`)
      (`BlackboardComponent.SetValueAsBool` (`AIBlueprintHelperLibrary.GetBlackboard` null) "bFightEnded" true))))

(event `self.ReceiveBeginPlay`
  (`self.RunBehaviorTree` "/Game/Characters/BigTortoise/AI/BigTortoise_BT.BigTortoise_BT"))

(event `self.AIPerception.OnTargetPerceptionUpdated`
  (params (Actor :type "Actor Object Reference") (Stimulus :type "AIStimulus Structure"))
  (`self.HandleSight` Actor Stimulus))

(fn `EndBossFight`
  (bind _asactor (cast `Actor` (`BlackboardComponent.GetValueAsObject` (`AIBlueprintHelperLibrary.GetBlackboard` null) "LeftArenaBound")))
  (`self.K2_DestroyActor` _asactor)
  (bind _asactor_2 (cast `Actor` (`BlackboardComponent.GetValueAsObject` (`AIBlueprintHelperLibrary.GetBlackboard` null) "RightArenaBound")))
  (`self.K2_DestroyActor` _asactor_2)
  (bind _asplayer_character_bp_c (cast `/Game/Characters/Player/Player_Character_BP_C` (`GameplayStatics.GetPlayerCharacter` 0)))
  (`/Game/UI/PlayerHUD_BP_UW.EndBossFight` (`/Game/Characters/Player/Player_Character_BP_C.HUD_REF` _asplayer_character_bp_c))
  (`/Game/Characters/Player/Player_Character_BP_C.AddPlayerScore` _asplayer_character_bp_c 1000))

(fn `HandleSight`
  (params (Actor :type "Actor Object Reference") (Stimulus :type "AIStimulus Structure"))
  (bind _returnvalue (`AIPerceptionSystem.GetSenseClassForStimulus` Stimulus))
  (if (== _returnvalue "/Script/AIModule.AISense_Sight")
    (if (== (`local.Actor`) (`GameplayStatics.GetPlayerCharacter` 0))
      (`BlackboardComponent.SetValueAsObject` (`self.Blackboard`) "PlayerTarget" (`GameplayStatics.GetPlayerCharacter` 0))
      (return)
      (else
        _)))
  (return))

(fn `UserConstructionScript`)